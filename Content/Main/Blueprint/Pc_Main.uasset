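; Main player controller that sets the custom mouse cursor and relays right-click input.
; On BeginPlay it runs CursorEvent, which creates a WDG_Cursor widget and assigns it as the default software cursor.
; MouseEvent swaps in a WDG_Cursor_2 widget the same way but is not called within this graph.
; Pressing the RightClick action invokes CallRightCLick.
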(event Custom|CursorEvent
  (bind _returnvalue (Game|GetPlayerController 0))
  ;[1 1 1] Mouse/cursor
  (bind _returnvalue_2 (UserInterface|CreateWidget "/Game/Main/Blueprint/Widget/Start/WDG_Cursor.WDG_Cursor_C" _returnvalue))
  (Class|PlayerController|SetMouseCursorWidget _returnvalue "Default" _returnvalue_2))

(event Custom|MouseEvent
  (bind _returnvalue (Game|GetPlayerController 0))
  ;[1 1 1] Mouse/cursor
  (bind _returnvalue_2 (UserInterface|CreateWidget "/Game/Main/Blueprint/Widget/Start/WDG_Cursor_2.WDG_Cursor_2_C" _returnvalue))
  (Class|PlayerController|SetMouseCursorWidget _returnvalue "Default" _returnvalue_2))

(event EventBeginPlay
  ;[1 1 1] Begin
  (CallFunction|CursorEvent))

(event Input|ActionEvents|InputActionRightClick
  (params (Key :type Key%20Structure :default "None"))
  (:Pressed
    (Default|CallRightCLick)))

(fn ConstructionScript)